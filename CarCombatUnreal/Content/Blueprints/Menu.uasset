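; Main menu actor with clickable components for Play, Exit, HowTo and Back.
; Play opens Example_Map and Exit quits the game.
; HowTo and Back both toggle visibility on the same set of buttons and five Line components, flipping between the menu and what appears to be a how-to screen.
; The swap relies on each component's initial visibility, with no explicit screen state.
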(event OnClicked(Play)
  (params (TouchedComponent :type Primitive%20Component%20Object%20Reference))
  (Game|OpenLevel(byName) "Example_Map"))

(event OnClicked(Exit)
  (params (TouchedComponent :type Primitive%20Component%20Object%20Reference))
  (Game|QuitGame 0 "Quit"))

(event OnClicked(HowTo)
  (params (TouchedComponent :type Primitive%20Component%20Object%20Reference))
  (Rendering|ToggleVisibility (Variables|Default|GetPlay) false))

(event OnClicked(Back)
  (params (TouchedComponent :type Primitive%20Component%20Object%20Reference))
  (Rendering|ToggleVisibility (Variables|Default|GetPlay) false))

(fn ConstructionScript)