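; HUD Blueprint that draws the Sedan pawn's speed, gear, health, remaining turret count and timer as screen text.
; DrawHUD derives X and Y ratios against a 1280x720 reference to place and scale each line.
; It reads preformatted strings from the owning Sedan, switching the gear color in reverse.
; Drawing only runs while the Sedan's IsInCar flag is false.
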(event EventDrawHUD
  (params (SizeX :type Integer) (SizeY :type Integer))
  ;[1 1 1] Calculate ratio from 720p
  (bind _assedan_c (Utilities|Casting|CastToSedan (Class|HUD|GetOwningPawn)))
  (if (not (Variables|/Game/Sedan/Sedan.Sedan_C|GetIsInCar _assedan_c))
    (Utilities|FlowControl|Sequence
      (:then_0
        (Variables|Default|SetHUDXRatio (/ (Math|Conversions|ToFloat(Integer) SizeX) 1.28e+03)))
      (:then_1
        (Variables|Default|SetHUDYRatio (/ (Math|Conversions|ToFloat(Integer) SizeY) 7.2e+02)))
      (:then_2
        ;[1 1 1] Print vehicle speed
        (bind _assedan_c_2 (Utilities|Casting|CastToSedan (Class|HUD|GetOwningPawn)))
        (HUD|DrawText (Variables|/Game/Sedan/Sedan.Sedan_C|GetSpeed%20Display%20String _assedan_c_2) "(R=1.000000,G=1.000000,B=1.000000,A=1.000000)" (* 1.05e+03 (Variables|Default|GetHUDXRatio)) (* 645.0 (Variables|Default|GetHUDYRatio)) "/Engine/EngineFonts/RobotoDistanceField.RobotoDistanceField" (* 1.4 (Variables|Default|GetHUDYRatio)) false)
        ;[1 1 1] Print vehicle gear
        (bind _assedan_c_3 (Utilities|Casting|CastToSedan (Class|HUD|GetOwningPawn)))
        (HUD|DrawText (Utilities|String|Append "Gear:" (Variables|/Game/Sedan/Sedan.Sedan_C|GetGear%20Display%20String _assedan_c_3)) (Math|Color|SelectColor (Variables|/Game/Sedan/Sedan.Sedan_C|GetGearDisplayReverseColor _assedan_c_3) (Variables|/Game/Sedan/Sedan.Sedan_C|GetGearDisplayColor _assedan_c_3) (Variables|/Game/Sedan/Sedan.Sedan_C|GetInReverseGear _assedan_c_3)) (* 1.05e+03 (Variables|Default|GetHUDXRatio)) (* 675.0 (Variables|Default|GetHUDYRatio)) "/Engine/EngineFonts/RobotoDistanceField.RobotoDistanceField" (* 1.4 (Variables|Default|GetHUDYRatio)) false)
        ;[1 1 1] Update Health
        (bind _assedan_c_4 (Utilities|Casting|CastToSedan (Class|HUD|GetOwningPawn)))
        (HUD|DrawText (Utilities|String|Append "Health: " (Variables|/Game/Sedan/Sedan.Sedan_C|GetPlayer%20Health%20String _assedan_c_4)) "(R=1.000000,G=1.000000,B=1.000000,A=1.000000)" (* 5e+02 (Variables|Default|GetHUDXRatio)) (* 0.0 (Variables|Default|GetHUDYRatio)) 0 (* 1.4 (Variables|Default|GetHUDYRatio)) false)
        ;[1 1 1] Turret Count
        (bind _assedan_c_5 (Utilities|Casting|CastToSedan (Class|HUD|GetOwningPawn)))
        (HUD|DrawText (Utilities|String|Append "Turrets Remaining:" (Variables|/Game/Sedan/Sedan.Sedan_C|GetTurret%20Count%20String _assedan_c_5)) "(R=1.000000,G=1.000000,B=1.000000,A=1.000000)" (* 0.0 (Variables|Default|GetHUDXRatio)) (* 0.0 (Variables|Default|GetHUDYRatio)) 0 (* 1.4 (Variables|Default|GetHUDYRatio)) false)
        (bind _assedan_c_6 (Utilities|Casting|CastToSedan (Class|HUD|GetOwningPawn)))
        (HUD|DrawText (Utilities|String|Append "Time: " (Variables|/Game/Sedan/Sedan.Sedan_C|GetTimerString _assedan_c_6)) "(R=1.000000,G=1.000000,B=1.000000,A=1.000000)" (* 1.05e+03 (Variables|Default|GetHUDXRatio)) (* 0.0 (Variables|Default|GetHUDYRatio)) 0 (* 1.4 (Variables|Default|GetHUDYRatio)) false)))))

(fn ConstructionScript)