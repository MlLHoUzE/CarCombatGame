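; Turret actor that tracks and shoots at the player's pawn within attack range, and can be destroyed by player projectiles.
; Each tick it checks range, smoothly rotates its top toward the player with clamped pitch, and spawns bullets at the barrel socket, throttled by a Delay.
; Tagged projectile hits drain health until it explodes with sound and particles.
; BeginPlay also sets a turret count text.
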(event Custom|Fire%20Weapons
  ;[1 1 1] Fire Weapons
  (if (Variables|Default|GetEnemyInRange)
    (Utilities|FlowControl|Delay (Variables|TurretSettings|GetFireInterval))
    (Game|SpawnActorfromClass "/Game/Blueprints/Bullet.Bullet_C" (Transformation|GetSocketTransform (Variables|Default|GetTurret_Barrel) "Barrel" "RTS_World") false 0)))

(event Custom|Update%20Rotation
  (bind _returnvalue (Game|Player|GetPlayerPawn 0))
  (bind _turret_top (Variables|Default|GetTurret_Top))
  (bind _returnvalue_2 (Transformation|GetWorldLocation _turret_top))
  (bind _returnvalue_3 (Transformation|GetActorLocation _returnvalue))
  (bind _returnvalue_4 (Math|Rotator|FindLookatRotation _returnvalue_2 _returnvalue_3))
  (bind (_pitch _yaw) (Class|KismetMathLibrary|BreakRot _returnvalue_4))
  ;[1 1 1] Update Rotation
  (if (Variables|Default|GetEnemyInRange)
    (Transformation|SetWorldRotation (Variables|Default|GetTurret_Top) (Math|Interpolation|RInterpTo (Transformation|GetWorldRotation (Variables|Default|GetTurret_Top)) (Class|KismetMathLibrary|MakeRot (Math|Float|ClampAngle (- _pitch (Variables|TurretSettings|GetBarrelLength)) -3e+01 35.0) _yaw 0.0) (Variables|Default|GetDeltaTime) (Variables|TurretSettings|GetRotationSpeed)) false)))

(event Custom|Update%20Range
  ;[1 1 1] Update Range
  (bind _returnvalue (Transformation|GetDistanceTo self (Game|Player|GetPlayerPawn 0)))
  (if (<= _returnvalue (Variables|TurretSettings|GetAttackRange))
    (Variables|Default|SetEnemyInRange true)
    (else
      (Variables|Default|SetEnemyInRange false))))

(event EventTick
  (params (DeltaSeconds :type Float%20%28single-precision%29))
  ;[1 1 1] Game Loop
  (Variables|Default|SetDeltaTime DeltaSeconds)
  (CallFunction|UpdateRange)
  (CallFunction|UpdateRotation)
  (CallFunction|FireWeapons))

(event EventBeginPlay
  (Rendering|Components|TextRender|SetText (Variables|Default|GetInCarTurrets) (Variables|Default|GetTurret%20Count%20String)))

(event EventHit
  (params (MyComp :type Primitive%20Component%20Object%20Reference) (Other :type Actor%20Object%20Reference) (OtherComp :type Primitive%20Component%20Object%20Reference) (bSelfMoved :type Boolean) (HitLocation :type Vector :default "0, 0, 0") (HitNormal :type Vector :default "0, 0, 0") (NormalImpulse :type Vector :default "0, 0, 0") (Hit :type Hit%20Result%20Structure%20%28by%20ref%29))
  ;[1 1 1] Health
  (if (Actor|ActorHasTag Other "PlayerProjectile")
    (Variables|TurretSettings|SetHealth (Math|Float|Clamp(Float) (- (Variables|TurretSettings|GetHealth) 1e+01) 0.0 1e+02))
    (if (<= (Variables|TurretSettings|GetHealth) 0.0)
      (Audio|PlaySoundatLocation "/Game/StarterContent/Audio/Collapse01.Collapse01" (Transformation|GetActorLocation))
      (Effects|SpawnEmitteratLocation "/Game/StarterContent/Particles/P_Explosion2.P_Explosion2" (Transformation|GetActorLocation))
      (Actor|DestroyActor))))

(fn ConstructionScript)